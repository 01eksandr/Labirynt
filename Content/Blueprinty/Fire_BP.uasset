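; Fire actor that makes its point light flicker.
; On BeginPlay, a timeline's Flicker track scales the Light value to drive the point light's intensity.
; A GetAngle function yaws the actor toward the player camera like a billboard, ignoring height, but the looping timer meant to call it is disconnected and never runs.
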(event `self.ReceiveBeginPlay`
  (bind (_direction _flicker) (`Timeline|Timeline_0`)
    (:`Update`
      (`LightComponent.SetIntensity` (`self.PointLight`) (* (`self.Light`) _flicker)))))

(fn `getAngle`
  (`self.K2_SetActorRotation` (`KismetMathLibrary.Conv_VectorToRotator` (`KismetMathLibrary.Normal` (* (- (`PlayerCameraManager.GetCameraLocation` (`GameplayStatics.GetPlayerCameraManager` 0)) (`self.K2_GetActorLocation`)) (1.0 1.0 0.0))))))

(fn `UserConstructionScript`)